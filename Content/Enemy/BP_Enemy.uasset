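; Stationary enemy that waits crouched until a ThirdPersonCharacter enters its trigger box, then stands and attacks it.
; Crouching and standing halve and double the capsule half-height.
; Tick turns the enemy's yaw toward the target and, at FireRate intervals, spawns BP_Fireball from the gun's Muzzle socket aimed at it.
; A fireball hit ragdolls the mesh; Start, run on BeginPlay, clears the target and restores the mesh to the capsule.
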(event `self.ReceiveBeginPlay`
  (`self.Start`))

(event `self.ReceiveTick`
  (params (DeltaSeconds :type "Float (single-precision)"))
  (`self.RotateTowardsTarget`)
  (if (>= (- (`GameplayStatics.GetTimeSeconds`) (`self.LastFired`)) (`self.FireRate`))
    (`self.Fire`)
    (set `self.LastFired` (`GameplayStatics.GetTimeSeconds`))))

(event `RotateTowardsTarget`
  (bind _target (`self.Target`))
  (bind (_returnvalue_roll _returnvalue_pitch _returnvalue_yaw) (`KismetMathLibrary.BreakRotator` (`KismetMathLibrary.FindLookAtRotation` (`self.K2_GetActorLocation`) (`self.K2_GetActorLocation` _target))))
  (`/Engine/EditorBlueprintResources/StandardMacros.IsValid` _target
    (:`Is Valid`
      (`self.K2_SetActorRotation` (`KismetMathLibrary.MakeRotator` 0.0 0.0 _returnvalue_yaw)))))

(event `self.Box.OnComponentBeginOverlap`
  (params (OverlappedComponent :type "PrimitiveComponent Object Reference") (OtherActor :type "Actor Object Reference") (OtherComp :type "PrimitiveComponent Object Reference") (OtherBodyIndex :type Integer) (bFromSweep :type Boolean) (SweepResult :type "HitResult Structure (by ref)"))
  (bind _asthird_person_character (cast `/Game/ThirdPersonCPP/Blueprints/ThirdPersonCharacter` OtherActor))
  (`self.Uncrouch`)
  (set `self.Target` _asthird_person_character))

(event `Crouch`
  (bind _capsule (`self.Capsule`))
  (`CapsuleComponent.SetCapsuleHalfHeight` _capsule (/ (`CapsuleComponent.GetScaledCapsuleHalfHeight` _capsule) 2.0) true))

(event `Uncrouch`
  (bind _capsule (`self.Capsule`))
  (`CapsuleComponent.SetCapsuleHalfHeight` _capsule (* (`CapsuleComponent.GetScaledCapsuleHalfHeight` _capsule) 2.0) true))

(event `Fire`
  (bind _target (`self.Target`))
  (bind _returnvalue (`SceneComponent.GetSocketLocation` (`self.Gun`) "Muzzle"))
  (`/Engine/EditorBlueprintResources/StandardMacros.IsValid` _target
    (:`Is Valid`
      (`|SpawnActorFromClass` "/Game/FPWeapon/Projectile/Fireball/BP_Fireball.BP_Fireball_C" (`KismetMathLibrary.MakeTransform` _returnvalue (`KismetMathLibrary.FindLookAtRotation` _returnvalue (`self.K2_GetActorLocation` _target))) "AlwaysSpawn" "OverrideRootScale" self null))))

(event `self.Capsule.OnComponentHit`
  (params (HitComponent :type "PrimitiveComponent Object Reference") (OtherActor :type "Actor Object Reference") (OtherComp :type "PrimitiveComponent Object Reference") (NormalImpulse :type "Vector Structure") (Hit :type "HitResult Structure (by ref)"))
  (`KismetSystemLibrary.PrintString` "Enemy hit")
  (cast `/Game/FPWeapon/Projectile/Fireball/BP_Fireball` OtherActor)
  (`PrimitiveComponent.SetSimulatePhysics` (`self.SkeletalMesh`) true))

(event `Start`
  (bind _skeletalmesh (`self.SkeletalMesh`))
  (`KismetSystemLibrary.PrintString` "Start  enemy")
  (set `self.Target` null)
  (`SceneComponent.K2_AttachToComponent` (`self.SkeletalMesh`) (`self.Capsule`) "None" "KeepRelative" "KeepRelative" "KeepRelative" true)
  (`self.Crouch`)
  (`PrimitiveComponent.SetSimulatePhysics` _skeletalmesh false)
  (`SceneComponent.K2_SetRelativeLocationAndRotation` _skeletalmesh (0.0 0.0 -97.0) (struct :`Yaw` -90.0) false true)
  (`SceneComponent.K2_SetRelativeLocationAndRotation` (`self.SkeletalMesh`) (0.0 0.0 -97.0) (struct :`Yaw` -90.0) false true)
  (`KismetSystemLibrary.PrintString` (`KismetStringLibrary.Conv_VectorToString` (`SceneComponent.K2_GetComponentLocation` (`self.SkeletalMesh`)))))

(fn `UserConstructionScript`)